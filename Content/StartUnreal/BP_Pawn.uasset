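; BP_Pawn is a basic input-test pawn that moves, looks around and prints debug messages.
; Axis inputs offset the actor along its forward and right vectors without sweep or delta-time scaling.
; LookUP drives controller yaw and LookRight drives pitch, opposite to what their names suggest.
; Tick feeds ShowTimeSec, which accumulates delta time and prints each new whole second; BeginPlay, W and EnterInput also print.
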(event EventBeginPlay
  (Development|PrintString "Play" true true "(R=1.000000,G=0.166081,B=0.195929,A=1.000000)"))

(event EventTick
  (params (DeltaSeconds :type Float%20%28single-precision%29))
  (CallFunction|ShowTimeSec DeltaSeconds))

(event Input|ActionEvents|InputActionEnterInput
  (params (Key :type Key%20Structure :default "None"))
  (:Pressed
    (Development|PrintString "Enter press")))

(event Input|AxisEvents|InputAxisLookUP
  (params (AxisValue :type Float%20%28single-precision%29))
  ;[1 1 1] 마우스 x 축 움직임
  (Pawn|Input|AddControllerYawInput AxisValue))

(event Input|AxisEvents|InputAxisLookRight
  (params (AxisValue :type Float%20%28single-precision%29))
  ;[1 1 1] 마우스 y축 움직임
  (Pawn|Input|AddControllerPitchInput AxisValue))

(event Input|AxisEvents|InputAxisMoveRight
  (params (AxisValue :type Float%20%28single-precision%29))
  ;[1 1 1] 좌우로 움직임
  (Transformation|AddActorWorldOffset (* (Transformation|GetActorRightVector) (* AxisValue 1e+01))))

(event Input|AxisEvents|InputAxisMoveFoward
  (params (AxisValue :type Float%20%28single-precision%29))
  ;[1 1 1 1 20] 앞쪽으로 움직임
  (Transformation|AddActorWorldOffset (* (Transformation|GetActorForwardVector) (* AxisValue 1e+01))))

(event Input|KeyboardEvents|W
  (params (Key :type Key%20Structure :default "None"))
  (:Pressed
    (Development|PrintString "W key press")))

(fn ConstructionScript)

(fn ShowTimeSec
  (params (DeltaSeconds :type Float%20%28single-precision%29))
  (bind _output_get (Variables|Default|SetTotalDeltaSeconds (+ DeltaSeconds (Variables|Default|GetTotalDeltaSeconds))))
  (if (not (== (Variables|Default|GetBeforeInt) (Math|Float|Floor _output_get)))
    (Development|PrintString (Utilities|String|Append "Total Seconds : " (Utilities|String|ToString(Integer) (Math|Float|Floor _output_get))))
    (Variables|Default|SetBeforeInt (Math|Float|Floor _output_get))))